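; BP_Catapult is a physics-driven catapult that launches cannonballs with a spoon arm moved by a PhysicsConstraint angular drive.
; Shoot, allowed only when ready, sets a stiff drive toward a raised pitch target to swing the spoon.
; Reload swings it back with a weaker drive, then after a delay spawns a BP_Cannonball at the spawn point and marks it ready.
; Both first toggle the spoon's physics simulation off and on to reset it.
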(event Custom|Shoot
  (if (Variables|Default|GetbIsReadyToShoot)
    (bind _physicsconstraint (Variables|Default|GetPhysicsConstraint)
      (:then
        (CallFunction|ResetPhysic (Variables|Default|GetSpoonMesh))
        (Class|PhysicsConstraintComponent|SetAngularDriveParams _physicsconstraint 1e+04 0.0 0.0)
        (Class|PhysicsConstraintComponent|SetAngularOrientationTarget _physicsconstraint (Math|Rotator|MakeRotator 0.0 35.0 0.0))
        (Variables|Default|SetbIsReadyToShoot false))
      (:else))))

(event Custom|Reload
  (bind _physicsconstraint (Variables|Default|GetPhysicsConstraint)
    (:then
      (CallFunction|ResetPhysic (Variables|Default|GetSpoonMesh))
      (Class|PhysicsConstraintComponent|SetAngularDriveParams _physicsconstraint 1e+03 0.0 0.0)
      (Class|PhysicsConstraintComponent|SetAngularOrientationTarget _physicsconstraint (Math|Rotator|MakeRotator 0.0 -35.0 0.0))
      (Utilities|FlowControl|Delay 2.0)
      (Game|SpawnActorfromClass "/Game/HW_03/Blueprints/Cannonball/BP_Cannonball.BP_Cannonball_C" (Transformation|GetWorldTransform (Variables|Default|GetSpawnCannonBallPoint)) "AlwaysSpawn" "MultiplyWithRoot" 0 0)
      (Variables|Default|SetbIsReadyToShoot true))
    (:else)))

(event EventBeginPlay
  (Variables|Default|SetStartedSpoonTransform (Transformation|GetRelativeTransform (Variables|Default|GetSpoonMesh))))

(fn ConstructionScript)

(fn ResetPhysic
  (params (InComponent :type Primitive%20Component%20Object%20Reference))
  (Physics|SetSimulatePhysics InComponent false)
  (Physics|SetSimulatePhysics InComponent true))